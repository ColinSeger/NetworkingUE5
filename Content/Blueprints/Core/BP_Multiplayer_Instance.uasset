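; Game instance built on Advanced Steam Sessions that handles hosting, leaving and joining multiplayer sessions.
; Hosting creates a session, then opens ThirdPersonMap as a listen server.
; Leaving destroys any existing session, then loads the Menu level.
; Steam invites, both accepted and merely received, destroy the current session and join the invited one on success.
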(event `HostSession`
  ; Session Hosting
  (`CreateSessionCallbackProxyAdvanced.CreateAdvancedSession` :`PlayerController` (`GameplayStatics.GetPlayerController` 0) :`PublicConnections` 10 ; Is Avalible Since We Are Using Advanced Steam Sessions (And Inheriting From It's Game Instance)
    (:`OnSuccess`
      (set `PlayerController.bShowMouseCursor` false (`GameplayStatics.GetPlayerController` 0))
      (`GameplayStatics.OpenLevelBySoftObjectPtr` "/Game/ThirdPerson/Maps/ThirdPersonMap.ThirdPersonMap" true "?listen") ; The Option "?listen" is required to make a listen server
    )
    (:`OnFailure`
      (`KismetSystemLibrary.PrintString` "Failed to open session" true true (struct :`R` 1.0 :`A` 1.0) 20.0 "SessionError"))))

(event `OnLeaveSession`
  ; Leave Session Handling
  (bind _sessionstate (`AdvancedSessionsLibrary.GetSessionState`))
  (switch `EBPOnlineSessionState` _sessionstate
    (:`NoSession`
      (`GameplayStatics.OpenLevelBySoftObjectPtr` "/Game/Maps/Menu.Menu" :!label _label))
    (:`Creating`
      (`DestroySessionCallbackProxy.DestroySession` null :!label _label_2
        (:`OnSuccess`
          (goto _label))
        (:`OnFailure`
          (`KismetSystemLibrary.PrintString` "Failed to leave session" true true (struct :`R` 1.0 :`G` 0.208265 :`B` 0.218212 :`A` 1.0) 5.0))))
    (:`Pending`
      (goto _label_2))
    (:`Starting`
      (goto _label_2))
    (:`InProgress`
      (goto _label_2))
    (:`Ending`
      (goto _label_2))
    (:`Ended`
      (goto _label_2))))

(event `self.OnSessionInviteAccepted`
  (params (LocalPlayerNum :type Integer) (PersonInvited :type "BPUniqueNetId Structure") (SessionToJoin :type "BlueprintSessionResult Structure (by ref)"))
  (bind _returnvalue (`GameplayStatics.GetPlayerController` LocalPlayerNum))
  ; Steam Overlay Handling
  (`DestroySessionCallbackProxy.DestroySession` _returnvalue
    (:`OnSuccess`
      (`JoinSessionCallbackProxy.JoinSession` _returnvalue SessionToJoin
        (:`OnSuccess`
          (`KismetSystemLibrary.PrintString` "Joined Succesfully" true true (struct :`G` 0.66 :`B` 1.0 :`A` 1.0) 20.0))
        (:`OnFailure`
          (`KismetSystemLibrary.PrintString` "Failed To Join Session" true true (struct :`R` 1.0 :`B` 0.057804 :`A` 1.0) 20.0))))))

(event `self.OnSessionInviteReceived`
  (params (LocalPlayerNum :type Integer) (PersonInviting :type "BPUniqueNetId Structure") (AppId :type String) (SessionToJoin :type "BlueprintSessionResult Structure (by ref)"))
  (bind _returnvalue (`GameplayStatics.GetPlayerController` LocalPlayerNum))
  ; Steam Overlay Handling
  (`DestroySessionCallbackProxy.DestroySession` _returnvalue
    (:`OnSuccess`
      (`JoinSessionCallbackProxy.JoinSession` _returnvalue SessionToJoin))))